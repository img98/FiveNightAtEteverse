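; BP_MonsterSpawner is a placed actor that periodically spawns random monsters at its own transform in the FNAE VR game.
; On BeginPlay it binds to the FNAEVRGameMode game start and game over dispatchers.
; StartSpawnTimer runs DoSpawn on a looping timer with the first wait halved by a negative start delay, and StopSpawn clears it.
; DoSpawn picks a class from MonsterArray and passes Destination to the new monster.
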(event EventBeginPlay
  (CallFunction|BindGameMode))

(fn ConstructionScript)

(fn StartSpawnTimer
  (Utilities|Time|SetTimerbyFunctionName 0 "DoSpawn" (Variables|Default|GetSpawnInterval) true false (* (* (Variables|Default|GetSpawnInterval) -1.0) 0.5)))

(fn BindGameMode
  (bind _asfnaevrgame_mode (Utilities|Casting|CastToFNAEVRGameMode (Game|GetGameMode)))
  (Utilities|FlowControl|Sequence
    (:then_0
      (EventDispatchers|BindEventtoEventDispatcherGameStart _asfnaevrgame_mode (EventDispatchers|CreateEvent :!event StartSpawnTimer)))
    (:then_1
      (EventDispatchers|BindEventtoEventDispatcherGameOver _asfnaevrgame_mode (EventDispatchers|CreateEvent :!event StopSpawn)))))

(fn StopSpawn
  (if (Class|KismetSystemLibrary|TimerExists 0 "DoSpawn")
    (Utilities|Time|ClearTimerbyFunctionName 0 "DoSpawn")))

(fn DoSpawn
  (bind _monsterarray (Variables|Default|GetMonsterArray))
  (Game|SpawnActorfromClass (Utilities|Array|Get(acopy) _monsterarray (Math|Random|RandomIntegerinRange 0 (- (Utilities|Array|Length _monsterarray) 1))) (Transformation|GetActorTransform self) "Undefined" "MultiplyWithRoot" 0 (Variables|Default|GetDestination) 0))